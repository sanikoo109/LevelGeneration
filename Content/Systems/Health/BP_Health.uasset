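; BP_Health tracks a health value and handles incoming damage, with an optional linked armor object absorbing hits first.
; TakeDamage subtracts from ArmorRef when valid and passes only the unabsorbed remainder to health, otherwise applying full damage.
; AddHealth routes changes through SetHealth and returns the actual delta.
; SetHealth clamps between zero and MaxHealth and fires OnChangeHealth only when the value changes.
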(event Custom|SetHealth
  (params (Value :type Float%20%28single-precision%29))
  (bind _maxhealth (Variables|Default|GetMaxHealth))
  (bind _returnvalue (Math|Float|Clamp(Float) Value 0.0 _maxhealth))
  (if (!= _returnvalue (Variables|Default|GetCurrentHealth))
    (bind _output_get (Variables|Default|SetCurrentHealth _returnvalue))
    (Default|CallOnChangeHealth _output_get)))

(event Custom|TakeDamage
  (params (Damage :type Float%20%28single-precision%29))
  (Utilities|IsValid (Variables|Default|GetArmorRef)
    (:Is%20Valid
      (bind _addvalue (Default|AddArmor (Variables|Default|GetArmorRef) (* Damage -1.0)))
      (if (> (+ Damage _addvalue) 0.0)
        (CallFunction|AddHealth (* (+ Damage _addvalue) -1.0))))
    (:Is%20Not%20Valid
      (CallFunction|AddHealth (* Damage -1.0)))))

(fn ConstructionScript)

(fn AddHealth
  (params (Value :type Float%20%28single-precision%29))
  (LocalVariables|SetPrevHealth (Variables|Default|GetCurrentHealth))
  (CallFunction|SetHealth (+ (Variables|Default|GetCurrentHealth) Value))
  (return (- (Variables|Default|GetCurrentHealth) (LocalVariables|GetPrevHealth))))