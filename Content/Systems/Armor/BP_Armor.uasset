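; BP_Armor tracks an armor value kept between zero and MaxValue.
; SetArmor clamps the requested value and, only when it differs from the current one, stores it and fires OnChangeArmor with the new amount.
; AddArmor applies a relative change through SetArmor and returns the amount actually applied after clamping.
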(event Custom|SetArmor
  (params (Value :type Float%20%28single-precision%29))
  (bind _maxvalue (Variables|Default|GetMaxValue))
  (bind _returnvalue (Math|Float|Clamp(Float) Value 0.0 _maxvalue))
  (if (!= _returnvalue (Variables|Default|GetCurrentValue))
    (bind _output_get (Variables|Default|SetCurrentValue _returnvalue))
    (Default|CallOnChangeArmor _output_get)))

(fn ConstructionScript)

(fn AddArmor
  (params (Value :type Float%20%28single-precision%29))
  (LocalVariables|SetPrevValue (Variables|Default|GetCurrentValue))
  (CallFunction|SetArmor (+ (Variables|Default|GetCurrentValue) Value))
  (return (- (Variables|Default|GetCurrentValue) (LocalVariables|GetPrevValue))))