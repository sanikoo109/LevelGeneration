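; BP_Door is a swinging door actor that other code drives through Open and Close events.
; Both events play or reverse a timeline at a rate derived from OpenTime or CloseTime, lerping the door mesh's relative rotation up to MaxRotation.
; SetOpen records the open state and immediately toggles the Box collision, disabling it when open and restoring query and physics when closed.
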(event Custom|Open
  (CallFunction|SetOpen true)
  (Components|Timeline|SetPlayRate (Variables|Default|GetOpenCloseTimeline) (/ 1.0 (Variables|Default|GetOpenTime)))
  (bind _driver (Timeline|OpenCloseTimeline Play)
    (:Update
      (Transformation|SetRelativeRotation (Variables|Default|GetDoorMesh) (Math|Rotator|Lerp(Rotator) "0, 0, 0" (Variables|Default|GetMaxRotation) _driver true) false false))))

(event Custom|Close
  (CallFunction|SetOpen false)
  (Components|Timeline|SetPlayRate (Variables|Default|GetOpenCloseTimeline) (/ 1.0 (Variables|Default|GetCloseTime)))
  (bind _driver (Timeline|OpenCloseTimeline Reverse)
    (:Update
      (Transformation|SetRelativeRotation (Variables|Default|GetDoorMesh) (Math|Rotator|Lerp(Rotator) "0, 0, 0" (Variables|Default|GetMaxRotation) _driver true) false false))))

(fn ConstructionScript)

(fn SetOpen
  (params (IsOpen :type Boolean))
  (bind _output_get (Variables|Default|SetIsOpen IsOpen))
  (Collision|SetCollisionEnabled (Variables|Default|GetBox) (select _output_get "NoCollision" "QueryAndPhysics")))